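; BP_MenuGameMode is a game mode, apparently for the menu, that shows a debug readout of the chosen player's deathmatch record.
; Each Tick it casts the game instance to BP_FPSGameInstance and looks up ChosenPlayerName in PlayersProfileData.
; It prints the name with frags, deaths, suicides and score, using a zero-duration PrintString refreshed every frame.
; BeginPlay and the construction script are empty.
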(event `self.ReceiveTick`
  (params (DeltaSeconds :type "Float (single-precision)"))
  (bind _asbp_fpsgame_instance (cast `/Game/Blueprints/BP_FPSGameInstance` (`GameplayStatics.GetGameInstance`)))
  (bind _chosenplayername (`FPSGameInstance.ChosenPlayerName` _asbp_fpsgame_instance))
  (bind (_frags _deaths _suicides _score) (break `DeathmatchScore` (`.DMScore` (break `PlayerProfileData` (`BlueprintMapLibrary.Map_Find` (`FPSGameInstance.PlayersProfileData` _asbp_fpsgame_instance) _chosenplayername)))))
  (`KismetSystemLibrary.PrintString` (`KismetStringLibrary.Concat_StrStr` (`KismetStringLibrary.Concat_StrStr` _chosenplayername " has ") (`KismetStringLibrary.Concat_StrStr` " Frags : " (`KismetStringLibrary.Conv_IntToString` _frags) " Deaths : " (`KismetStringLibrary.Conv_IntToString` _deaths) " Suicides : " (`KismetStringLibrary.Conv_IntToString` _suicides) " Score : " (`KismetStringLibrary.Conv_IntToString` _score))) true true (struct :`G` 0.66 :`B` 1.0 :`A` 1.0) 0.0))

(fn `UserConstructionScript`)