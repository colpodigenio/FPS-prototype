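; BP_Projectile is a projectile actor that spawns a surface-dependent explosion effect and leaves a debug trail of its path.
; PlayImpactEffect calls SetImpactEffect, which picks the green explosion for Head and Body physical surfaces and the standard explosion otherwise.
; It then spawns that emitter, scaled down, at the actor's location.
; Tick draws a long-lived debug point at the current position every frame.
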(event `self.PlayImpactEffect`
  (params (ImpactPhysMat :type "PhysicalMaterial Object Reference"))
  (`self.SetImpactEffect` ImpactPhysMat)
  (`GameplayStatics.SpawnEmitterAtLocation` (`self.ImpactEffect`) (`self.K2_GetActorLocation`) (struct) (0.1 0.1 0.1)))

(event `self.ReceiveTick`
  (params (DeltaSeconds :type "Float (single-precision)"))
  (`KismetSystemLibrary.DrawDebugPoint` (`self.K2_GetActorLocation`) 5.0 (struct) 50.0))

(fn `SetImpactEffect`
  (params (PhysicalMaterial :type "PhysicalMaterial Object Reference"))
  (switch `EPhysicalSurface` (`PhysicalMaterial.SurfaceType` PhysicalMaterial)
    (:`SurfaceType_Default`
      (set `self.ImpactEffect` "/Game/StarterContent/Particles/P_Explosion.P_Explosion"))
    (:`SurfaceType1`
      (set `self.ImpactEffect` "/Game/StarterContent/Particles/P_ExplosionGreen.P_ExplosionGreen" :!label _label))
    (:`SurfaceType2`
      (goto _label))))

(fn `UserConstructionScript`)