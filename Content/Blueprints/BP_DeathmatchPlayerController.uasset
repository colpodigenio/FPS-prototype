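; BP_DeathmatchPlayerController is a deathmatch player controller that manages a scoreboard overlay.
; On BeginPlay it creates a W_Scoreboard widget, adds it to the viewport and keeps it hidden.
; The ShowScoreboard input action shows the widget while held and hides it on release.
; A debug print of the pawn's name is left unconnected and never runs.
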(event `self.ReceiveBeginPlay`
  (bind _returnvalue (`|CreateWidget` "/Game/UI/W_Scoreboard.W_Scoreboard_C"))
  (bind _output_get (set `self.ScoreboardRef` _returnvalue))
  (`UserWidget.AddToViewport` _output_get 0)
  (`Widget.SetVisibility` (`self.ScoreboardRef`) "Hidden"))

(event `self.ReceiveTick`
  (params (DeltaSeconds :type "Float (single-precision)")))

(event `InputAction|ShowScoreboard`
  (params (Key :type "Key Structure"))
  (bind _scoreboardref (`self.ScoreboardRef`))
  (:`Pressed`
    (`Widget.SetVisibility` _scoreboardref "Visible"))
  (:`Released`
    (`Widget.SetVisibility` _scoreboardref "Hidden")))

(fn `UserConstructionScript`)