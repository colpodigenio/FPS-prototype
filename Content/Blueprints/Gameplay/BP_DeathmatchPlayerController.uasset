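; Player controller for deathmatch that owns the player's HUD, scoreboard and in-game menu widgets.
; BeginPlay creates all three, hiding the scoreboard and menu and pointing the HUD at the controlled FPS character.
; Possess and UnPossess retarget, show or hide the HUD, while held input toggles the scoreboard.
; Esc pauses the game and opens the menu with UI-only input and a visible cursor.
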(event `self.ReceiveBeginPlay`
  ;[1 1 1] Create ScoreBoard
  (bind _returnvalue (`|CreateWidget` "/Game/UI/W_Scoreboard.W_Scoreboard_C"))
  (bind _output_get (set `self.ScoreboardRef` _returnvalue))
  (`UserWidget.AddToViewport` _output_get 0)
  (`Widget.SetVisibility` (`self.ScoreboardRef`) "Hidden")
  (`WidgetBlueprintLibrary.SetInputMode_GameOnly` self)
  ;[1 1 1] Create IngameMenu
  (bind _returnvalue_2 (`|CreateWidget` "/Game/UI/W_IngameMenu.W_IngameMenu_C"))
  (bind _output_get_2 (set `self.IngameMenuRef` _returnvalue_2))
  (`UserWidget.AddToViewport` _output_get_2 0)
  (`Widget.SetVisibility` _output_get_2 "Hidden")
  ;[1 1 1] Create HUD
  (bind _returnvalue_3 (`|CreateWidget` "/Game/UI/W_HUD.W_HUD_C" (`GameplayStatics.GetPlayerController` 0)))
  (bind _output_get_3 (set `self.PlayerHUD` _returnvalue_3))
  (`UserWidget.AddToViewport` _output_get_3 0)
  (bind _asbp_fpscharacter (cast `/Game/Blueprints/BP_FPSCharacter` (`self.K2_GetPawn`)))
  (set `/Game/UI/W_HUD.OwnerRef` _asbp_fpscharacter (`self.PlayerHUD`)))

(event `self.ReceiveTick`
  (params (DeltaSeconds :type "Float (single-precision)")))

(event `InputAction|Show Scoreboard`
  (params (Key :type "Key Structure"))
  (:`Pressed`
    (`self.ShowScoreboard`))
  (:`Released`
    (`self.HideScoreboard`)))

(event `InputAction|Esc`
  (params (Key :type "Key Structure"))
  (:`Pressed`
    (`GameplayStatics.SetGamePaused` true)
    (`WidgetBlueprintLibrary.SetInputMode_UIOnlyEx` self null)
    (`Widget.SetVisibility` (`self.IngameMenuRef`) "Visible")
    (set `self.bShowMouseCursor` true)))

(event `self.ReceiveEndPlay`
  (params (EndPlayReason :type "EEndPlayReason Enum" :default "Destroyed"))
  (`WidgetBlueprintLibrary.SetInputMode_UIOnlyEx` self null))

(event `self.ShowScoreboard`
  (`Widget.SetVisibility` (`self.ScoreboardRef`) "Visible"))

(event `self.HideScoreboard`
  (`Widget.SetVisibility` (`self.ScoreboardRef`) "Hidden"))

(event `self.ReceivePossess`
  (params (PossessedPawn :type "Pawn Object Reference"))
  (bind _playerhud (`self.PlayerHUD`))
  (bind _asbp_fpscharacter (cast `/Game/Blueprints/BP_FPSCharacter` PossessedPawn))
  (`/Engine/EditorBlueprintResources/StandardMacros.IsValid` _playerhud
    (:`Is Valid`
      (set `/Game/UI/W_HUD.OwnerRef` _asbp_fpscharacter _playerhud)
      (`Widget.SetVisibility` (`self.PlayerHUD`) "Visible"))))

(event `self.ReceiveUnPossess`
  (params (UnpossessedPawn :type "Pawn Object Reference"))
  (bind _playerhud (`self.PlayerHUD`))
  (`/Engine/EditorBlueprintResources/StandardMacros.IsValid` _playerhud
    (:`Is Valid`
      (`Widget.SetVisibility` _playerhud "Hidden"))))

(fn `UserConstructionScript`)