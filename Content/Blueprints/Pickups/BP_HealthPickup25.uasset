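; Health pickup Blueprint, judging by its name, with no healing or pickup logic in these graphs.
; BeginPlay stores a random color in NewVar0, taking each RGB channel from a separate random unit vector.
; Debug drawing and printing of the actor name and Mesh visibility are disconnected and never run.
; The overlap event is disabled and the construction script is empty.
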(event `self.ReceiveBeginPlay`
  (set `self.NewVar_0` (make `LinearColor` (.x (`KismetMathLibrary.RandomUnitVector`)) (.y (`KismetMathLibrary.RandomUnitVector`)) (.z (`KismetMathLibrary.RandomUnitVector`)) 1.0)))

(fn `UserConstructionScript`)