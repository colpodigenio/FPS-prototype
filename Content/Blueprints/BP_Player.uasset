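; Player Blueprint that owns the HUD, a weapon inventory and a health component.
; BeginPlay shows the HUD, spawns a socket-attached assault rifle as current weapon in the inventory, then applies damage to itself.
; SpawnWeaponFromPickup spawns and attaches a weapon by type and hides the player mesh; its assault rifle branch never reaches its return.
; Tick prints health and armor as debug output.
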(event `self.ReceiveBeginPlay`
  (bind _mesh (`self.Mesh`))
  (`|ExecutionSequence`
    (:`then_0`
      (bind _returnvalue (`|CreateWidget` "/Game/UI/HUD.HUD_C" (`GameplayStatics.GetPlayerController` 0)))
      (bind _output_get (set `self.PlayerHUD` _returnvalue))
      (`UserWidget.AddToViewport` _output_get 0))
    (:`then_1`
      ;[1 1 1] Spawn default weapon
      (`/Engine/EditorBlueprintResources/StandardMacros.IsValid` _mesh
        (:`Is Valid`
          (bind _returnvalue_2 (`|SpawnActorFromClass` "/Game/Blueprints/BP_AssaultRifle.BP_AssaultRifle_C" (`SceneComponent.GetSocketTransform` _mesh "InventorySocket" "RTS_World") "AlwaysSpawn" "OverrideRootScale" self self))
          (`self.K2_AttachToComponent` _returnvalue_2 (`self.Mesh`) "AssaultRifle" "SnapToTarget" "SnapToTarget" "SnapToTarget" false)
          (set `self.CurrentWeapon` _returnvalue_2)
          (`BlueprintMapLibrary.Map_Add` (`self.WeaponInventory`) (enumliteral `EWeaponType` "AssaultRifle") _returnvalue_2))))
    (:`then_2`
      (`HealthComponent.ApplyDamage` (`self.HealthComponent`) 50))))

(event `self.ReceiveTick`
  (params (DeltaSeconds :type "Float (single-precision)"))
  (bind _healthcomponent (`self.HealthComponent`))
  (`KismetSystemLibrary.PrintString` (`KismetStringLibrary.Concat_StrStr` (`KismetStringLibrary.Conv_IntToString` (`HealthComponent.GetHealth` _healthcomponent)) "::" (`KismetStringLibrary.Conv_IntToString` (`HealthComponent.GetArmor` _healthcomponent))) true true (struct :`G` 0.66 :`B` 1.0 :`A` 1.0) 0.0))

(fn `SpawnWeaponFromPickup`
  (params (WeaponType :type "EWeaponType Enum" :default "None"))
  (returns (ReturnValue :type "Weapon Object Reference"))
  (bind _returnvalue (`KismetMathLibrary.MakeTransform` (0.0 0.0 0.0)))
  (bind _mesh (`self.Mesh`))
  (bind _mesh_2 (`self.Mesh`))
  (bind _mesh_3 (`self.Mesh`))
  (switch `EWeaponType` WeaponType
    (:`AssaultRifle`
      (`/Engine/EditorBlueprintResources/StandardMacros.IsValid` (`self.Mesh`)
        (:`Is Valid`
          (bind _returnvalue_2 (`|SpawnActorFromClass` "/Game/Blueprints/BP_AssaultRifle.BP_AssaultRifle_C" _returnvalue "AlwaysSpawn" "OverrideRootScale" self self))
          (`SceneComponent.SetVisibility` _mesh_2 false false)
          (`self.K2_AttachToComponent` _returnvalue_2 _mesh_2 "AssaultRifle" "SnapToTarget" "SnapToTarget" "SnapToTarget" false))))
    (:`Shotgun`
      (`/Engine/EditorBlueprintResources/StandardMacros.IsValid` (`self.Mesh`)
        (:`Is Valid`
          (bind _returnvalue_3 (`|SpawnActorFromClass` "/Game/Blueprints/BP_Shotgun.BP_Shotgun_C" _returnvalue "AlwaysSpawn" "OverrideRootScale" self self))
          (`SceneComponent.SetVisibility` _mesh_3 false false)
          (`self.K2_AttachToComponent` _returnvalue_3 _mesh_3 "Shotgun" "SnapToTarget" "SnapToTarget" "SnapToTarget" false)
          (return _returnvalue_3))))
    (:`RocketLauncher`
      (`/Engine/EditorBlueprintResources/StandardMacros.IsValid` (`self.Mesh`)
        (:`Is Valid`
          (bind _returnvalue_4 (`|SpawnActorFromClass` "/Game/Blueprints/BP_RocketLauncher.BP_RocketLauncher_C" _returnvalue "AlwaysSpawn" "OverrideRootScale" self self))
          (`SceneComponent.SetVisibility` _mesh false false)
          (`self.K2_AttachToComponent` _returnvalue_4 _mesh "RocketLauncher" "SnapToTarget" "SnapToTarget" "SnapToTarget" false)
          (return _returnvalue_4))))))

(fn `UserConstructionScript`)